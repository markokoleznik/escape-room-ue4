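; OpenableDoor_BP is a door actor that swings open and closed in response to its OpenDoor component's OnOpen and OnClose events.
; It caches its starting rotation at BeginPlay, then the DoorSwing timeline adds its OpenAngle track to that yaw on each update.
; Opening plays the timeline and closing reverses it.
; A Doorlock sound node is present but unconnected, so it never plays.
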(event OnOpen(OpenDoor)
  (bind _initialrotation (Variables|Default|GetInitialRotation))
  (bind (_roll _pitch _yaw) (Math|Rotator|BreakRotator _initialrotation))
  (bind _openangle (Timeline|Door%20Swing Play)
    (:Update
      (Transformation|SetActorRotation (Math|Rotator|MakeRotator _roll _pitch (+ _yaw _openangle))))))

(event OnClose(OpenDoor)
  (bind _initialrotation (Variables|Default|GetInitialRotation))
  (bind (_roll _pitch _yaw) (Math|Rotator|BreakRotator _initialrotation))
  (bind _openangle (Timeline|Door%20Swing Reverse)
    (:Update
      (Transformation|SetActorRotation (Math|Rotator|MakeRotator _roll _pitch (+ _yaw _openangle))))))

(event EventBeginPlay
  (Variables|Default|SetInitialRotation (Transformation|GetActorRotation)))

(fn ConstructionScript)